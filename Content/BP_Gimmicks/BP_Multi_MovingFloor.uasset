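; BP_Multi_MovingFloor is a multiplayer gimmick floor that moves only while at least two player characters overlap its Box.
; InterpToMovement starts with its component tick disabled; each Tick, the server counts overlapping BP_ThirdPersonCharacter actors and toggles that tick to run or pause movement.
; The server also sets Glowing, whose RepNotify swaps the Cube material to show the active state.
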(event EventBeginPlay
  (Components|Tick|SetComponentTickEnabled (Variables|Default|GetInterpToMovement) false))

(event Collision|EventActorBeginOverlap
  (params (OtherActor :type Actor%20Object%20Reference)))

(event EventTick
  (params (DeltaSeconds :type Float%20%28single-precision%29))
  (Networking|SwitchHasAuthority
    (:Authority
      (if (>= (Utilities|Array|Length (Collision|GetOverlappingActors (Variables|Default|GetBox) "/Game/ThirdPerson/Blueprints/BP_ThirdPersonCharacter.BP_ThirdPersonCharacter_C" :!class /Script/Engine.PrimitiveComponent)) 2)
        (Components|Tick|SetComponentTickEnabled (Variables|Default|GetInterpToMovement) true)
        (Variables|Default|SetbGlowing true)
        (else
          (Components|Tick|SetComponentTickEnabled (Variables|Default|GetInterpToMovement) false)
          (Variables|Default|SetbGlowing false))))))

(fn ConstructionScript)

(fn OnRepBGlowing
  (if (Variables|Default|GetbGlowing)
    (Rendering|Material|SetMaterial (Variables|Default|GetCube) 0 "/Game/BP_Gimmicks/MT_MultiMovingFloor.MT_MultiMovingFloor")
    (else
      (Rendering|Material|SetMaterial (Variables|Default|GetCube) 0 "/Game/FirstPerson/Blueprints/AI/Turrel/cano.cano"))))