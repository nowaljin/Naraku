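; BP_EnemyPatroler_kadai is a patrolling enemy that explodes on contact with the player.
; From BeginPlay it loops AI MoveTo through Waypoints, pausing after each successful arrival except when wrapping to the first.
; Overlapping its Box drains the character's Stamina, spawns an explosion with sound and destroys the enemy.
; Projectile damage and score logic exists but is disconnected, so it never runs.
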(event OnComponentBeginOverlap(Box)
  (params (OverlappedComponent :type Primitive%20Component%20Object%20Reference) (OtherActor :type Actor%20Object%20Reference) (OtherComp :type Primitive%20Component%20Object%20Reference) (OtherBodyIndex :type Integer) (bFromSweep :type Boolean) (SweepResult :type Hit%20Result%20Structure%20%28by%20ref%29))
  ;[0.15 0.15 0.15 0.5] Player Hit
  (bind _asbp_third_person_character (Utilities|Casting|CastToBP_ThirdPersonCharacter OtherActor))
  (Variables|/Game/ThirdPerson/Blueprints/BP_ThirdPersonCharacter.BP_ThirdPersonCharacter_C|Setstamina _asbp_third_person_character (- (Variables|/Game/ThirdPerson/Blueprints/BP_ThirdPersonCharacter.BP_ThirdPersonCharacter_C|Getstamina _asbp_third_person_character) 2e+01))
  (Effects|SpawnEmitteratLocation "/Game/StarterContent/Particles/P_Explosion.P_Explosion" (Transformation|GetActorLocation) "0, 0, 0" "2.000000,2.000000,2.000000")
  (Audio|PlaySound2D "/Game/Map/Music/SC_EnemyBump.SC_EnemyBump" 1.0 1.0 0.0 0 0)
  (Actor|DestroyActor))

(event Custom|Patrol
  ;[0.15 0.15 0.15 0.5] Patrolling
  (AI|AIMoveTo self "0, 0, 0" (Utilities|Array|Get(acopy) (Variables|Default|GetWaypoints) (Variables|Default|GetCurrentWaypoint)) 5.0 false
    (:OnSuccess
      (Math|Integer|IncrementInt (Variables|Default|GetCurrentWaypoint)
        (:%20%20
          (if (>= (Variables|Default|GetCurrentWaypoint) (Utilities|Array|Length (Variables|Default|GetWaypoints)))
            (Variables|Default|SetCurrentWaypoint 0)
            (else
              (Utilities|FlowControl|Delay 3.0)))
          (CallFunction|Patrol))))))

(event EventBeginPlay
  (CallFunction|Patrol))

(fn ConstructionScript)